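; AI controller that runs the AI_BT behavior tree and tracks a target enemy through AI perception.
; On perception updates, only AIChar_BP or PlayerChar_BP actors are considered.
; A successful sense stores the actor as TargetEnemy and writes it to the EnemyActor blackboard key, while a failed sense clears both.
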(event `self.ReceiveBeginPlay`
  (`self.RunBehaviorTree` "/Game/AI/AI_BT.AI_BT"))

(event `self.AIPerception.OnTargetPerceptionUpdated`
  (params (Actor :type "Actor Object Reference") (Stimulus :type "AIStimulus Structure"))
  (bind _returnvalue (`AIBlueprintHelperLibrary.GetBlackboard` null))
  (cast `/Game/AI/AIChar_BP` Actor
    (:`then`
      _)
    (:`CastFailed`
      (cast `/Game/Player/PlayerChar_BP` Actor)))
  (if (`.bSuccessfullySensed` (break `AIStimulus` Stimulus))
    (bind _output_get (set `self.TargetEnemy` Actor))
    (`/Engine/EditorBlueprintResources/StandardMacros.IsValid` _returnvalue
      (:`Is Valid`
        (`BlackboardComponent.SetValueAsObject` _returnvalue "EnemyActor" _output_get)))
    (else
      (set `self.TargetEnemy` null)
      (`BlackboardComponent.SetValueAsObject` _returnvalue "EnemyActor" null))))

(fn `UserConstructionScript`)